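; BP_Satellites animates a swarm of instanced-mesh satellites orbiting around a planet radius.
; The construction script adds the instances on an evenly spaced ring and stores a phase for each.
; Tick advances the phases and rebuilds each transform on a randomly tilted circular orbit, varying speed, radius, roll and scale.
; Resetting the random stream every frame replays the same random values, avoiding stored per-satellite orbit parameters.
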(event `self.ReceiveBeginPlay`)

(event `self.ReceiveTick`
  (params (DeltaSeconds :type "Float (single-precision)"))
  (bind _phases (`self.Phases`))
  (bind _instancedstaticmesh (`self.InstancedStaticMesh`))
  (bind _newvar_1 (`self.NewVar_1`))
  (bind _returnvalue (`KismetMathLibrary.RandomFloatInRangeFromStream` 0.7 1.3 _newvar_1))
  (`KismetMathLibrary.ResetRandomStream` _newvar_1)
  (for _index (range (`InstancedStaticMeshComponent.GetInstanceCount` _instancedstaticmesh))
    (bind _output (`|GetArrayItem` _phases _index))
    (`KismetArrayLibrary.Array_Set` _phases _index (+ _output (/ DeltaSeconds _returnvalue)))
    (bind _returnvalue_2 (* _output (`self.RotationSpeed`)))
    (bind _returnvalue_3 (`KismetMathLibrary.RotateAngleAxis` (* (`KismetMathLibrary.MakeVector` (`KismetMathLibrary.Cos` _returnvalue_2) (`KismetMathLibrary.Sin` _returnvalue_2)) (* _returnvalue (`self.PlanetRadius`))) 180.0 (`KismetMathLibrary.RandomUnitVectorFromStream` _newvar_1)))
    (`InstancedStaticMeshComponent.UpdateInstanceTransform` _instancedstaticmesh _index (`KismetMathLibrary.MakeTransform` _returnvalue_3 (`KismetMathLibrary.ComposeRotators` (`KismetMathLibrary.MakeRotator` (`KismetMathLibrary.RandomFloatInRangeFromStream` 0.0 180.0 _newvar_1)) (`KismetMathLibrary.Conv_VectorToRotator` _returnvalue_3)) (`KismetMathLibrary.Conv_DoubleToVector` (`KismetMathLibrary.RandomFloatInRangeFromStream` 0.7 1.3 _newvar_1))) false true false)))

(fn `UserConstructionScript`
  (bind _satellitecount (`self.SatelliteCount`))
  (for _index (range 1 (+ _satellitecount 1))
    (bind _returnvalue (* (/ (`KismetMathLibrary.Conv_IntToDouble` _index) _satellitecount) 6.28))
    (`KismetArrayLibrary.Array_Add` (`self.Phases`) _returnvalue)
    (`InstancedStaticMeshComponent.AddInstance` (`self.InstancedStaticMesh`) (`KismetMathLibrary.MakeTransform` (* (`KismetMathLibrary.MakeVector` (`KismetMathLibrary.Cos` _returnvalue) (`KismetMathLibrary.Sin` _returnvalue)) (`self.PlanetRadius`)) (`KismetMathLibrary.RandomRotator` true)) false)))